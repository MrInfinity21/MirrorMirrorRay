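; A Blueprint function library of shared helpers for rotator math, timeline timing, interaction direction checks and mesh coloring.
; Rotators are added or subtracted per component, and timeline play rate is derived from a desired duration.
; Interaction direction comes from the impact normal's dominant local horizontal axis, while side uses the sign of a 2D cross product.
; A color lookup feeds a dynamic material instance that sets BaseColor on a mesh's first material slot.
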(fn RotatorAddition
  (params (Rotator1 :type Rotator) (Rotator2 :type Rotator))
  (return (Math|Rotator|MakeRotator (+ (.roll Rotator1) (.roll Rotator2)) (+ (.pitch Rotator1) (.pitch Rotator2)) (+ (.yaw Rotator1) (.yaw Rotator2)))))

(fn RotatorSubtraction
  (params (RotatorToSubtractFrom :type Rotator) (RotatorToSubtract :type Rotator))
  (return (Math|Rotator|MakeRotator (- (.roll RotatorToSubtractFrom) (.roll RotatorToSubtract)) (- (.pitch RotatorToSubtractFrom) (.pitch RotatorToSubtract)) (- (.yaw RotatorToSubtractFrom) (.yaw RotatorToSubtract)))))

(fn SetNewTimelinePlayRate
  (params (Timeline :type Timeline%20Component%20Object%20Reference) (NewDuration :type Float%20%28double-precision%29))
  (Components|Timeline|SetPlayRate Timeline (Math|Float|SafeDivide (Components|Timeline|GetTimelineLength Timeline) NewDuration)))

(fn GetInteractionDirection
  (params (ImpactNormal :type Vector) (InteractedActor :type Actor%20Object%20Reference))
  (bind _returnvalue (Transformation|GetActorRotation InteractedActor))
  (bind _returnvalue_2 (Math|Vector|UnrotateVector ImpactNormal _returnvalue))
  (bind _returnvalue_3 (Math|Vector|DotProduct _returnvalue_2 "1.000000,0.000000,0.000000"))
  (bind _returnvalue_4 (Math|Vector|DotProduct _returnvalue_2 "0.000000,1.000000,0.000000"))
  (if (>= (Math|Float|Absolute(Float) _returnvalue_3) (Math|Float|Absolute(Float) _returnvalue_4))
    (if (>= _returnvalue_3 0.0)
      (return "NewEnumerator1")
      (else
        (return "NewEnumerator0")))
    (elif (>= _returnvalue_4 0.0)
      (return "NewEnumerator2")
      (else
        (return "NewEnumerator3")))))

(fn GetInteractionSide
  (params (CallingActor :type Actor%20Object%20Reference) (CallingActorForward :type Vector) (InteractedActor :type Actor%20Object%20Reference))
  (return (>= (Class|KismetMathLibrary|CrossProduct2D (Math|Conversions|ToVector2D(Vector) (- (Transformation|GetActorLocation CallingActor) (Transformation|GetActorLocation InteractedActor))) (Math|Conversions|ToVector2D(Vector) (Math|Vector|Normalize CallingActorForward))) 0.0)))

(fn GetColor
  (params (ColorDesired :type E_Colors%20Enum :default "NewEnumerator0"))
  (return (.Value (Utilities|Map|Find (LocalVariables|GetAvailableColors) ColorDesired))))

(fn SetMatBaseColor
  (params (Mesh :type Primitive%20Component%20Object%20Reference) (Color :type E_Colors%20Enum :default "NewEnumerator0"))
  (bind _returnvalue (Rendering|Material|CreateDynamicMaterialInstance 0 (Rendering|Material|GetMaterial Mesh 0) "None" :!class /Script/Engine.KismetMaterialLibrary))
  (Rendering|Material|SetVectorParameterValue _returnvalue "BaseColor" (CallFunction|GetColor Color) :!class /Script/Engine.MaterialInstanceDynamic)
  (Rendering|Material|SetMaterial Mesh 0 _returnvalue))