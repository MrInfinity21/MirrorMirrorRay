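; Light emitter for a laser puzzle that casts a colored beam through mirrors and color blocks to activate door triggers.
; On BeginPlay it loops multi line traces, spawning a stretched BP_LaserBeam per hit segment and skipping the last-hit actor.
; Mirrors reflect the ray up to a maximum count, color blocks recolor it, and other hits end it, passing the color to door triggers.
; RecalculateBeams destroys the tracked beams and traces again.
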(event EventBeginPlay
  (CallFunction|CreateNewBeams))

(fn ConstructionScript)

(fn CreateNewBeams
  (Utilities|FlowControl|Sequence
    (:then_0
      ;[0.15 0.15 0.15 0.5] Set RayStart & RayEnd
      (bind _output_get (LocalVariables|SetRayStart (.location (Transformation|GetActorTransform))))
      (LocalVariables|SetRayEnd (+ _output_get (* (Transformation|GetActorForwardVector) (Variables|Default|GetRaycastLength)))))
    (:then_1
      (Variables|Default|SetCurrentBeamColor (CallFunction|GetColor (Variables|Default|GetDefaultBeamColor))))
    (:then_2
      (while (and (not (LocalVariables|GetBlockerEncountered)) (< (LocalVariables|Getcounter) (Variables|Default|GetMaxReflections)))
        (bind (_outhits _returnvalue) (Collision|MultiLineTraceByChannel (LocalVariables|GetRayStart) (LocalVariables|GetRayEnd) "TraceTypeQuery3" false (Variables|Default|GetBeamList) "None"))
        (if _returnvalue
          (bind _array_element (Utilities|Array|ForEachLoopwithBreak _outhits :!label _label) ; Continue looping through hits until we hit a new object
            (:LoopBody
              (if (!= (LocalVariables|GetLastHItActor) (.HitActor (Collision|BreakHitResult _array_element)))
                (goto _label Break)))
            (:Completed
              (Utilities|FlowControl|Sequence
                (:then_0
                  (LocalVariables|SetLastHItActor (.HitActor (Collision|BreakHitResult _array_element)))
                  (LocalVariables|SetImpact%20Point (.ImpactPoint (Collision|BreakHitResult _array_element)))
                  (bind _output_get_2 (LocalVariables|SetCastRay (- (.ImpactPoint (Collision|BreakHitResult _array_element)) (.TraceStart (Collision|BreakHitResult _array_element)))))
                  (CallFunction|SpawnNewBeam (LocalVariables|GetRayStart) _output_get_2 (Variables|Default|GetCurrentBeamColor)))
                (:then_1
                  (Utilities|Casting|CastToBP_Mirror (.HitActor (Collision|BreakHitResult _array_element)) ; 4. Check if hit object is reflective
                    (:then
                      (Utilities|CalculateReflectedRay (LocalVariables|GetImpact%20Point) (.Normal (Collision|BreakHitResult _array_element))))
                    (:CastFailed
                      (bind _asbp_color_block (Utilities|Casting|CastToBP_ColorBlock (.HitActor (Collision|BreakHitResult _array_element)))
                        (:then
                          (LocalVariables|SetRayStart (LocalVariables|GetImpact%20Point))
                          (Variables|Default|SetCurrentBeamColor (CallFunction|GetColor (Variables|/Game/Blueprints/BP_ColorBlock.BP_ColorBlock_C|GetBlockColor _asbp_color_block))))
                        (:CastFailed
                          (bind _asbp_door_trigger (Utilities|Casting|CastToBP_DoorTrigger (.HitActor (Collision|BreakHitResult _array_element))) ; Check if object is door trigger
                            (:then
                              (Default|ActivateTrigger _asbp_door_trigger (Variables|Default|GetCurrentBeamColor)))
                            (:CastFailed
                              _))
                          (LocalVariables|SetBlockerEncountered true) ; Stop creating beams
                        ))))))))
          (else
            (return)))))))

(fn SpawnNewBeam
  (params (Beam%20Start :type Vector) (Beam%20Vector :type Vector) (BeamColor :type Linear%20Color%20Structure))
  (bind _returnvalue (Game|SpawnActorfromClass "/Game/Blueprints/BP_LaserBeam.BP_LaserBeam_C" (Math|Transform|MakeTransform Beam%20Start (Math|Rotator|MakeRotfromZ Beam%20Vector) (Math|Vector|MakeVector 1.0 1.0 (/ (Math|Vector|VectorLength Beam%20Vector) 1e+02))) "Undefined" "MultiplyWithRoot" 0 0)) ; 2. Spawn new beam
  (Default|SetBeamEmissiveColor _returnvalue BeamColor)
  (Utilities|Array|AddUnique (Variables|Default|GetBeamList) _returnvalue) ; 3. Add to list
)

(fn RecalculateBeams
  (CallFunction|ClearBeams)
  (CallFunction|CreateNewBeams))

(fn ClearBeams
  (for _array_element (Variables|Default|GetBeamList)
    (Actor|DestroyActor _array_element))
  (Utilities|Array|Clear (Variables|Default|GetBeamList)))