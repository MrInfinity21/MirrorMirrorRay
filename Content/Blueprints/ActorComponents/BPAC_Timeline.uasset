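; Base actor component that imitates a timeline with a looping timer, for child Blueprints to define timed behaviour.
; StartTimeline calls the overridable CheckCanStart, which must set IsTimelineActive for the timer to begin at a DeltaTime interval.
; Each tick advances LerpTime and calls the overridable Behaviour, then clears the timer and active flag once Duration is reached.
; Both override functions are empty here, and StartTimeline does nothing while already active.
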(event Custom|TimelineActive
  (Variables|Default|SetLerpTime (+ (Variables|Default|GetLerpTime) (Variables|Default|GetDeltaTime)))
  ;[0.15 0.15 0.15 0.5] Overwrite
  (CallFunction|Behaviour)
  (if (>= (Variables|Default|GetLerpTime) (Variables|Default|GetDuration))
    (Utilities|Time|ClearandInvalidateTimerbyHandle (stale Custom|StartTimeline _returnvalue))
    (Variables|Default|SetIsTimelineActive false)))

(event Custom|StartTimeline
  (if (not (Variables|Default|GetIsTimelineActive))
    ;[0.15 0.15 0.15 0.5] Overwrite
    (CallFunction|CheckCanStart)
    (if (Variables|Default|GetIsTimelineActive)
      (Variables|Default|SetLerpTime 0.0)
      (bind _returnvalue (Utilities|Time|SetTimerbyEvent (delegate Custom|TimelineActive) (Variables|Default|GetDeltaTime) true)))))

(fn CheckCanStart)

(fn Behaviour)