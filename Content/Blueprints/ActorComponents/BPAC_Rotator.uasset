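; Actor component that rotates its owner in bounded steps, left or right, for the mirror and light puzzle.
; StartRotation stores the side and starts the timeline, while CheckCanStart activates it only if a rotation is set and the step counter is within bounds.
; Behaviour overrides the parent's to spread each step over Duration, calling ResetAllBeams on BP_FirstPersonGameMode with every increment, a project-specific coupling.
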(event Custom|StartRotation
  (params (Side :type Boolean))
  (Variables|Default|SetSideToRotate Side)
  (CallFunction|StartTimeline))

(event EventBeginPlay
  (Utilities|NegateInt (Variables|Default|GetRotationRightBound)
    (:%20%20
      ;[0.15 0.15 0.15 0.5] Unique to this Project - MirrorLightGamePuzzle
      (bind _asbp_first_person_game_mode (Utilities|Casting|CastToBP_FirstPersonGameMode (Game|GetGameMode)))
      (Variables|Default|SetRefGameMode _asbp_first_person_game_mode))))

(fn Behaviour
  (Class|Actor|AddActorWorldRotation (Components|GetOwner) (* (* (Variables|Default|GetDeltaRotator) (/ (Variables|Default|GetDeltaTime) (Variables|Default|GetDuration))) (Variables|Default|GetRotationDirection)))
  ;[0.15 0.15 0.15 0.5] Unique to this Project - MirrorLightPuzzleGame
  (Default|ResetAllBeams (Variables|Default|GetRefGameMode)))

(fn CheckCanStart
  (bind _rotationcount (Variables|Default|GetRotationCount))
  (Utilities|FlowControl|Sequence
    (:then_0
      (if (not (Utilities|Operators|NotEqual(!=) :A (Variables|Default|GetDeltaRotator)))
        (return)))
    (:then_1
      (if (Variables|Default|GetSideToRotate)
        (if (> (Variables|Default|GetRotationCount) (Variables|Default|GetRotationRightBound))
          (Math|Integer|DecrementInt _rotationcount
            (:%20%20
              (Variables|Default|SetRotationDirection 1)
              (Variables|Default|SetIsTimelineActive true :!label _label))))
        (elif (< (Variables|Default|GetRotationCount) (Variables|Default|GetRotationLeftBound))
          (Math|Integer|IncrementInt _rotationcount
            (:%20%20
              (Variables|Default|SetRotationDirection -1)
              (goto _label))))))))