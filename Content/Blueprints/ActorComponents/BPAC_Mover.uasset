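; Mover component for the mirror-light puzzle that slides its owning actor one grid step left, right, forward or back along world axes.
; Before starting the timeline move, it checks per-axis step counts against bounds and box-traces the owner's bounds for blockers.
; Step size can derive automatically from actor bounds.
; Each update applies a time-scaled world offset, unaffected by actor rotation, and has the game mode reset all beams.
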(event Custom|StartMovement
  (params (Direction :type E_Direction%20Enum :default "NewEnumerator2"))
  (Variables|Default|SetMovementDirection Direction)
  (CallFunction|StartTimeline))

(event EventBeginPlay
  (bind _returnvalue (Components|GetOwner))
  (bind _boxextent (Collision|GetActorBounds _returnvalue false false))
  (Utilities|FlowControl|Sequence
    (:then_0
      (bind _result (Math|Float|NegateFloat (.x (Variables|Default|GetMoverXBounds)))
        (:%20%20
          (Variables|Default|SetMoverXBounds (Math|Vector2D|MakeVector2D _result (.y (Variables|Default|GetMoverXBounds))))
          (bind _result_2 (Math|Float|NegateFloat (.x (Variables|Default|GetMoverYBounds)))
            (:%20%20
              (Variables|Default|SetMoverYBounds (Math|Vector2D|MakeVector2D _result_2 (.y (Variables|Default|GetMoverYBounds)))))))))
    (:then_1
      (if (Variables|Default|GetSetupDeltaMoverAutomatically)
        (Variables|Default|SetDeltaMover (Math|Vector2D|MakeVector2D (* (.x _boxextent) 2.0) (* (.y _boxextent) 2.0)))))
    (:then_2
      ;[0.15 0.15 0.15 0.5] Unique to this Project - MirrorLightGamePuzzle
      (bind _asbp_first_person_game_mode (Utilities|Casting|CastToBP_FirstPersonGameMode (Game|GetGameMode)))
      (Variables|Default|SetRefGameMode _asbp_first_person_game_mode))))

(fn CheckCanStart
  (bind _returnvalue (Components|GetOwner))
  (bind (_origin _boxextent) (Collision|GetActorBounds _returnvalue false false))
  (switch Utilities|FlowControl|Switch|SwitchonE_Direction (Variables|Default|GetMovementDirection)
    (:NewEnumerator2
      ;[0.15 0.15 0.15 0.5] Have we Hit Mover Limit in corresponding Direction
      (if (> (.y (Variables|Default|GetMoverCount)) (.x (Variables|Default|GetMoverYBounds)))
        (Variables|Default|SetMoverDirection "(X=0.000000,Y=-1.000000)")
        (Utilities|FlowControl|Sequence
          (:then_0
            ;[0.15 0.15 0.15 0.5] Check if there is something Blocking
            (bind _returnvalue_2 (Collision|BoxTraceByChannel _origin (+ _origin (* (Variables|Default|GetMoverDirection) (Variables|Default|GetDeltaMover))) _boxextent "0, 0, 0" "TraceTypeQuery1" false 0 "None" :!label _label))
            (if _returnvalue_2
              (return)
              (else
                (Variables|Default|SetIsTimelineActive true))))
          (:then_1
            (bind _result (Math|Float|DecrementFloat (.y (Variables|Default|GetMoverCount)))
              (:%20%20
                (Variables|Default|SetMoverCount (Math|Vector2D|MakeVector2D (.x (Variables|Default|GetMoverCount)) _result))))))
        (else
          (return))))
    (:NewEnumerator3
      (if (< (.y (Variables|Default|GetMoverCount)) (.y (Variables|Default|GetMoverYBounds)))
        (Variables|Default|SetMoverDirection "(X=0.000000,Y=1.000000)")
        (Utilities|FlowControl|Sequence
          (:then_0
            (goto _label))
          (:then_1
            (bind _result_2 (Math|Float|IncrementFloat (.y (Variables|Default|GetMoverCount)))
              (:%20%20
                (Variables|Default|SetMoverCount (Math|Vector2D|MakeVector2D (.x (Variables|Default|GetMoverCount)) _result_2))))))
        (else
          (return))))
    (:NewEnumerator0
      (if (< (.x (Variables|Default|GetMoverCount)) (.y (Variables|Default|GetMoverXBounds)))
        (Variables|Default|SetMoverDirection "(X=1.000000,Y=0.000000)")
        (Utilities|FlowControl|Sequence
          (:then_0
            (goto _label))
          (:then_1
            (bind _result_3 (Math|Float|IncrementFloat (.x (Variables|Default|GetMoverCount)))
              (:%20%20
                (Variables|Default|SetMoverCount (Math|Vector2D|MakeVector2D _result_3 (.y (Variables|Default|GetMoverCount))))))))
        (else
          (return))))
    (:NewEnumerator1
      (if (> (.x (Variables|Default|GetMoverCount)) (.x (Variables|Default|GetMoverXBounds)))
        (Variables|Default|SetMoverDirection "(X=-1.000000,Y=0.000000)")
        (Utilities|FlowControl|Sequence
          (:then_0
            (goto _label))
          (:then_1
            (bind _result_4 (Math|Float|DecrementFloat (.x (Variables|Default|GetMoverCount)))
              (:%20%20
                (Variables|Default|SetMoverCount (Math|Vector2D|MakeVector2D _result_4 (.y (Variables|Default|GetMoverCount))))))))
        (else
          (return))))))

(fn Behaviour
  (bind _duration (Variables|Default|GetDuration))
  (bind _deltamover (Variables|Default|GetDeltaMover))
  (bind _deltatime (Variables|Default|GetDeltaTime))
  (bind _moverdirection (Variables|Default|GetMoverDirection))
  (bind _returnvalue (/ _deltatime _duration))
  (bind _returnvalue_2 (* _deltamover _returnvalue))
  (Transformation|AddActorWorldOffset (Components|GetOwner) (Math|Vector|MakeVector (* (.x _returnvalue_2) (.x _moverdirection)) (* (.y _moverdirection) (.y _returnvalue_2)) 0.0))
  ;[0.15 0.15 0.15 0.5] Unique to this Project - MirrorLightPuzzleGame
  (Default|ResetAllBeams (Variables|Default|GetRefGameMode)))