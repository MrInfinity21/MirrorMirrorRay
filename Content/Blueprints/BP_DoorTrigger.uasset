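; BP_DoorTrigger is a color-keyed switch that opens a linked door when hit by a beam of the matching color.
; The construction script converts the required color setting into the trigger color and tints the switch mesh to show it.
; ActivateTrigger compares the incoming beam color to that trigger color and calls OpenDoor on the door only on an exact match.
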(fn ConstructionScript
  (bind _colorrequired (Variables|Default|GetColorRequired))
  (Variables|Default|SetColorToTrigger (CallFunction|GetColor _colorrequired))
  (CallFunction|SetMatBaseColor (Variables|Default|GetSwitchMesh) _colorrequired))

(fn ActivateTrigger
  (params (BeamColor :type Linear%20Color%20Structure))
  (if (== BeamColor (Variables|Default|GetColorToTrigger))
    (Default|OpenDoor (Variables|Default|GetDoor))))